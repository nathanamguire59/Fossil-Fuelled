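; Enemy character for an FPS that roams random navmesh points and chases the player once pawn sensing sees a pawn.
; Hit damage scales by the physical material's DestructibleDamageThresholdScale, while explosive damage falls off linearly with distance.
; Both feed HealthUpdate and spawn randomly offset screen-space damage numbers; direct hits also show hit markers and flag headshots by surface type.
; Death enables ragdoll physics with a weapon-scaled impulse away from the player.
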(event `self.ReceiveBeginPlay`
  (`|ExecutionSequence`
    (:`then_0`
      ;[1 0 0] Reference to Player
      (bind _asbp_player (cast `/Game/FPSGame/Character/BP_Player` (`GameplayStatics.GetPlayerCharacter` 0)))
      (set `self.Player` _asbp_player))
    (:`then_1`
      ;[1 0 0] Enemy AI
      (`self.Roam`))))

(event `/Game/FPSGame/Interfaces/BPI_TakeDamage.EnemyTakeDamage`
  (params (WeaponStats :type "/Game/FPSGame/Data/S_WeaponStats Structure") (HitResult :type "HitResult Structure"))
  (bind (_bblockinghit _binitialoverlap _time _distance _location _impactpoint _normal _impactnormal _physmat _hitactor _hitcomponent _hitbonename) (`GameplayStatics.BreakHitResult` HitResult))
  ;[1 0 0] Enemy taking damage
  (if (not (`self.isDead?`))
    (bind _calculateddamage (`self.CalculateDamage` (`.Damage_2_9351663E4278E736465ABE8579C1497E` (break `/Game/FPSGame/Data/S_WeaponStats` WeaponStats)) HitResult))
    (bind _isdead_ (`self.HealthUpdate` _calculateddamage))
    (bind _output_get (set `self.isDead?` _isdead_))
    (if _output_get
      (`self.EnemyDeath` _impactnormal _hitbonename))
    (`self.DamageNumbers` _calculateddamage _impactnormal (`|EnumEquality` (`PhysicalMaterial.SurfaceType` _physmat) "SurfaceType1"))
    (`/Engine/EditorBlueprintResources/StandardMacros.IsValid` (`self.HitMarkerReference`)
      (:`Is Valid`
        (`Widget.RemoveFromParent` (`self.HitMarkerReference`)) ; Removes previous marker if another hit occurs before the first disappears
      )
      (:`Is Not Valid`
        _))
    (bind _returnvalue (`|CreateWidget` "/Game/FPSGame/UI/HitMarkers.HitMarkers_C" null (`self.isDead?`)))
    (bind _output_get_2 (set `self.HitMarkerReference` _returnvalue))
    (`UserWidget.AddToViewport` _output_get_2 0)))

(event `self.DamageNumbers`
  (params (Damage :type "Float (single-precision)") (ImpactLocation :type "Vector Structure") (`isHeadshot?` :type Boolean))
  (bind (_x _y) (`KismetMathLibrary.BreakVector2D` (`WidgetLayoutLibrary.ProjectWorldLocationToWidgetPosition` (`GameplayStatics.GetPlayerController` 0) ImpactLocation)))
  (bind _returnvalue (`|CreateWidget` "/Game/FPSGame/UI/DamageNumbers.DamageNumbers_C" null Damage `isHeadshot?`))
  (`Widget.SetRenderTranslation` (`/Game/FPSGame/UI/DamageNumbers.SizeBox_49` _returnvalue) (`KismetMathLibrary.MakeVector2D` (+ (+ _x -100.0) (`KismetMathLibrary.RandomFloatInRange` -25.0 150.0)) (+ (+ _y -100.0) (`KismetMathLibrary.RandomFloatInRange` 0.0 50.0))))
  (`UserWidget.AddToViewport` _returnvalue 0))

(event `/Game/FPSGame/Interfaces/BPI_TakeDamage.TakeRadiusDamage`
  (params (HitResult :type "HitResult Structure") (WeaponStats :type "/Game/FPSGame/Data/S_WeaponStats Structure"))
  (bind (_damage _impactradius) (break `/Game/FPSGame/Data/S_WeaponStats` WeaponStats))
  (bind (_bblockinghit _binitialoverlap _time _distance _location _impactpoint _normal _impactnormal _physmat _hitactor _hitcomponent _hitbonename) (`GameplayStatics.BreakHitResult` HitResult))
  ;[1 0 0] Enemy takes damage from explosives
  (if (not (`self.isDead?`))
    (bind _radiusdamageapplied (`self.CalculateRadiusDamage` _damage _impactradius _impactpoint))
    (bind _isdead_ (`self.HealthUpdate` _radiusdamageapplied))
    (if _isdead_
      (`self.EnemyDeath` _impactpoint _hitbonename))
    (`self.DamageNumbers` _radiusdamageapplied _impactpoint)))

(event `Roam`
  ;[1 0 0] AI Roam
  (`|AIMoveTo` self (`NavigationSystemV1.K2_GetRandomLocationInNavigableRadius` (`self.K2_GetActorLocation`) 2000.0 null null) null
    (:`OnSuccess`
      (`KismetSystemLibrary.Delay` 0.5)
      (`self.Roam`))))

(event `ChasePlayer`
  ;[1 0 0] AI Chase
  (`|AIMoveTo` self (0.0 0.0 0.0) (`GameplayStatics.GetPlayerCharacter` 0) :!label _label
    (:`OnSuccess`
      (`KismetSystemLibrary.Delay` 1.0)
      (`self.ChasePlayer`))))

(event `self.PawnSensing.OnSeePawn`
  (params (Pawn :type "Pawn Object Reference"))
  ;[1 0 0] AI Chase
  (goto _label))

(fn `CalculateDamage`
  (params (Damage :type "Float (double-precision)") (HitResult :type "HitResult Structure"))
  (returns (CalculatedDamage :type "Float (double-precision)"))
  (locals (LocalDamage :type "Float (double-precision)"))
  (set `local.LocalDamage` Damage)
  (return (* (`local.LocalDamage`) (`PhysicalMaterial.DestructibleDamageThresholdScale` (`.PhysMat` (`GameplayStatics.BreakHitResult` HitResult))))))

(fn `CalculateRadiusDamage`
  (params (Damage :type "Float (double-precision)") (ImpactRadius :type "Float (double-precision)") (ImpactPoint :type "Vector Structure"))
  (returns (RadiusDamageApplied :type "Float (double-precision)"))
  (locals (LocalDamage :type "Float (double-precision)"))
  (set `local.LocalDamage` Damage)
  (return (`KismetMathLibrary.FClamp` (* (- 1.0 (/ (`KismetMathLibrary.VSize` (- ImpactPoint (`self.K2_GetActorLocation`))) ImpactRadius)) (`local.LocalDamage`)) 0.0 (`local.LocalDamage`))))

(fn `EnemyDeath`
  (params (HitLocation :type "Vector Structure") (BoneName :type Name))
  (bind _player (`self.Player`))
  (`|ExecutionSequence`
    (:`then_0`
      ;[1 0 0] Enabling Ragdoll Physics
      (`PrimitiveComponent.SetSimulatePhysics` (`self.Mesh`) true))
    (:`then_1`
      (`GameplayStatics.PlaySound2D` "/Game/FPSGame/Audio/kill-sound.kill-sound" 1.0 1.0 0.0 null null))
    (:`then_2`
      (`PrimitiveComponent.AddImpulseAtLocation` (`self.Mesh`) (* (`KismetMathLibrary.GetDirectionUnitVector` (`self.K2_GetActorLocation` _player) (`self.K2_GetActorLocation`)) (`/Game/FPSGame/Weapons/WeaponBase.KillImpulse` (`/Game/FPSGame/Character/BP_Player.CurrentWeapon` _player))) HitLocation BoneName)
      (`ActorComponent.K2_DestroyComponent` (`self.CapsuleComponent`)))))

(fn `HealthUpdate`
  (params (DamageApplied :type "Float (double-precision)"))
  (returns (`isDead?` :type Boolean))
  (locals (`LocalIsDead?` :type Boolean))
  (`|ExecutionSequence`
    (:`then_0`
      (if (>= DamageApplied (`self.CurrentHealth`))
        (set `local.LocalIsDead?` true)
        (set `self.CurrentHealth` 0.0)
        (else
          (set `self.CurrentHealth` (- (`self.CurrentHealth`) DamageApplied)))))
    (:`then_1`
      (return (`local.LocalIsDead?`)))))

(fn `UserConstructionScript`)