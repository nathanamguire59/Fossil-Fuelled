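; First-person shooter player character handling movement, damage, HUD creation and weapon use.
; Pickups found by a camera line trace supply ammo or weapons, which spawn onto arm sockets in six slots, with swaps toggling visibility.
; Firing and ammo math are delegated to the current weapon, while state flags gate shooting, reloading, aiming and sprinting.
; Timelines drive the reload arm dip and sprint stamina, which reverses to regenerate after a pause or exhaustion.
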(event `self.ReceiveBeginPlay`
  (`|ExecutionSequence`
    (:`then_0`
      ;[1 0 0] Creates Main HUD
      (bind _returnvalue (`|CreateWidget` "/Game/FPSGame/UI/MainHUD.MainHUD_C"))
      (bind _output_get (set `self.MainHUD` _returnvalue))
      (`UserWidget.AddToViewport` _output_get 0))))

(event `self.ReceiveAnyDamage`
  (params (Damage :type "Float (single-precision)") (DamageType :type "DamageType Object Reference") (InstigatedBy :type "Controller Object Reference") (DamageCauser :type "Actor Object Reference"))
  ;[1 0 0] Enemy Damages Player
  (set `self.CurrentHealth` (- (`self.CurrentHealth`) Damage)))

(event `Key|Seven`
  (params (Key :type "Key Structure"))
  ;[1 0 0] Weapon Swap Test
  (:`Pressed`
    (`KismetSystemLibrary.PrintString` (`KismetSystemLibrary.GetDisplayName` (`self.CurrentWeapon`)))))

(event `WeaponPickUp`
  (params (WeaponToSpawn :type "/Game/FPSGame/Weapons/WeaponBase Class Reference"))
  (bind _returnweapon (`self.SpawnWeapon` WeaponToSpawn))
  (`self.EquipWeapon` _returnweapon))

(event `EquipWeapon`
  (params (Weapon :type "/Game/FPSGame/Weapons/WeaponBase Object Reference"))
  (if (not (`self.isSwitchingWeapon?`))
    (if (`self.isReloading?`)
      (set `self.isReloading?` false))
    (set `self.isSwitchingWeapon?` true)
    (`self.HideAndShowWeaponMesh` Weapon)
    (set `self.Loadout` "NewEnumerator1")
    (`/Game/FPSGame/UI/Crosshair.CrosshairUpdate` (`/Game/FPSGame/UI/MainHUD.Crosshair` (`self.MainHUD`)))
    (`KismetSystemLibrary.Delay` 0.33) ; Allows time for weapon switch animation
    (set `self.isSwitchingWeapon?` false)
    (set `self.CanShoot?` true) ; Can't shoot while switching weapons
  ))

(event `Fire`
  (bind _currentweapon (`self.CurrentWeapon`))
  (bind _currentweapon_2 (`self.CurrentWeapon`))
  (if (`self.CanShoot?`)
    (if (`/Game/FPSGame/Weapons/WeaponBase.DoWeHaveAmmo?` _currentweapon_2)
      (`/Game/FPSGame/Weapons/WeaponBase.StartShooting` _currentweapon (`/Game/FPSGame/Weapons/WeaponBase.FireType` _currentweapon))
      (elif (`/Game/FPSGame/Weapons/WeaponBase.IsThereAmmoLeft?` _currentweapon_2)
        ;[1 0 0] Reloads weapon if there is reserev ammo
        (`self.Reload`)
        (else
          (`GameplayStatics.PlaySound2D` "/Game/UEAssets/ShooterGame/Sounds/Weapons/GrenadeLauncher/wav/sw_Wep_Launcher_Dryfire_01.sw_Wep_Launcher_Dryfire_01" 1.0 1.0 0.0 null null))))))

(event `Reload`
  (bind _currentweapon (`self.CurrentWeapon`))
  (if (`self.CanWeReload?`)
    (`|ExecutionSequence`
      (:`then_0`
        (set `self.isReloading?` true)
        (set `self.CanShoot?` false)
        (set `self.isAiming?` false)
        ;[1 0 0] Controls animations for reloading
        (bind (_direction _pulldown) (`Timeline|WeaponPullDown` :!via `PlayFromStart`)
          (:`Update`
            (if (`self.isReloading?`)
              (set `self.PulldownTimer` _pulldown)))
          (:`Finished`
            (`KismetSystemLibrary.Delay` (`/Game/FPSGame/Weapons/WeaponBase.ReloadTime` (`self.CurrentWeapon`)))
            (bind (_direction_2 _pullup) (`Timeline|WeaponPullUp` :!via `PlayFromStart`)
              (:`Update`
                (if (`self.isReloading?`)
                  (set `self.PulldownTimer` _pullup)
                  (`/Engine/EditorBlueprintResources/StandardMacros.DoOnce` false :!label _label
                    (:`Completed`
                      (`GameplayStatics.PlaySound2D` (`/Game/FPSGame/Weapons/WeaponBase.ReloadEndSound` (`self.CurrentWeapon`)) 1.0 1.0 0.0 null null)
                      (`KismetSystemLibrary.Delay` 1.0)
                      (goto _label :!via `Reset`)))))
              (:`Finished`
                (if (`self.isReloading?`)
                  (`/Game/FPSGame/Weapons/WeaponBase.ReloadCalculation` (`self.CurrentWeapon`)) ; Does Maths for Bullets
                  (set `self.isReloading?` false)
                  (set `self.CanShoot?` true)))))))
      (:`then_1`
        (if (not (`self.isSprinting?`))
          (set `CharacterMovementComponent.MaxWalkSpeed` (`self.MaxWalkSpeed`) (`self.CharacterMovement`))))
      (:`then_2`
        (`GameplayStatics.PlaySound2D` (`/Game/FPSGame/Weapons/WeaponBase.ReloadStartSound` (`self.CurrentWeapon`)) 1.0 1.0 0.0 null null)
        (if (`/Game/FPSGame/Weapons/WeaponBase.isShotgun?` (`self.CurrentWeapon`))
          (`/Game/FPSGame/Weapons/WeaponBase.ShotgunReloadPellets` _currentweapon)
          (`KismetSystemLibrary.Delay` (`/Game/FPSGame/Weapons/WeaponBase.ReloadTime` _currentweapon))
          (set `/Game/FPSGame/Weapons/WeaponBase.ReloadTime` 0.3 _currentweapon) ; Resetting back to the Default Time
        )))))

(event `InputAxis|MoveForward`
  (params (AxisValue :type "Float (single-precision)"))
  ;[1 0 0] WASD Movement Input
  (`self.AddMovementInput` (`KismetMathLibrary.GetForwardVector` (`KismetMathLibrary.MakeRotator` 0.0 0.0 (.yaw (`self.GetControlRotation`)))) AxisValue))

(event `InputAxis|MoveRight`
  (params (AxisValue :type "Float (single-precision)"))
  ;[1 0 0] WASD Movement Input
  (`self.AddMovementInput` (`KismetMathLibrary.GetRightVector` (`KismetMathLibrary.MakeRotator` 0.0 0.0 (.yaw (`self.GetControlRotation`)))) AxisValue))

(event `InputAction|Jump`
  (params (Key :type "Key Structure"))
  ;[1 0 0] Jump Action Event
  (:`Pressed`
    (`self.Jump`))
  (:`Released`
    (`self.StopJumping`)))

(event `self.ReceiveTick`
  (params (DeltaSeconds :type "Float (single-precision)"))
  ;[1 0 0] Checks to see if "W" key is released while sprinting
  (if (`self.HaveWeStoppedMoving?`)
    (`self.MovementStopped`) ; Connected to Timeline
  ))

(event `InputAction|Sprint`
  (params (Key :type "Key Structure"))
  ;[1 0 0] Sprint With Regenerating Stamina Bar
  (:`Pressed`
    (if (not (`self.isAiming?`))
      (if (not (`self.isReloading?`))
        (if (`self.AreWeExhausted?`)
          (`self.StartSprint`)
          (switch `/Game/FPSGame/Data/E_Loadout` (`self.Loadout`)
            (:`NewEnumerator0`
              (bind (_direction _staminaamount) (`Timeline|Stamina` :!label _label)
                (:`Update`
                  (bind _output_get (set `self.EnergyLevel` _staminaamount)))
                (:`Finished`
                  (if (== _output_get 0.0)
                    (`self.Exhausted`)))))
            (:`NewEnumerator1`
              (`/Game/FPSGame/Weapons/WeaponBase.StopShooting` (`self.CurrentWeapon`))
              (goto _label))))))))

(event `MovementStopped`
  ;[1 0 0] Sprint With Regenerating Stamina Bar
  (if (not (`self.isExhausted?`))
    (`|ExecutionSequence`
      (:`then_0`
        (`self.StopSprint`)
        (goto _label :!via `Stop`))
      (:`then_1`
        (`KismetSystemLibrary.Delay` (`self.StaminaRegenPause`))
        (goto _label :!via `Reverse`)))))

(event `Exhausted`
  ;[1 0 0] Sprint With Regenerating Stamina Bar
  (set `self.isExhausted?` true)
  (`self.StopSprint`)
  (`KismetSystemLibrary.Delay` (`self.ExhaustedTimer`))
  (set `self.isExhausted?` false)
  (goto _label :!via `ReverseFromEnd`))

(event `Key|One`
  (params (Key :type "Key Structure"))
  (bind _weaponslot01 (`self.WeaponSlot01`))
  ;[1 0 0] Key Bindings to Equip Weapons After They've Been Initially Picked Up
  (:`Pressed`
    (if (`self.is1stSlotFilled?`)
      (if (not (== (`self.CurrentWeapon`) (`self.WeaponSlot01`)))
        (`self.EquipWeapon` _weaponslot01)
        (set `self.CurrentWeapon` _weaponslot01)
        (`/Game/FPSGame/UI/Crosshair.CrosshairUpdate` (`/Game/FPSGame/UI/MainHUD.Crosshair` (`self.MainHUD`)) :!label _label)))))

(event `Key|Two`
  (params (Key :type "Key Structure"))
  (bind _weaponslot02 (`self.WeaponSlot02`))
  ;[1 0 0] Key Bindings to Equip Weapons After They've Been Initially Picked Up
  (:`Pressed`
    (if (`self.is2ndSlotFilled?`)
      (if (not (== (`self.CurrentWeapon`) (`self.WeaponSlot02`)))
        (`self.EquipWeapon` _weaponslot02)
        (set `self.CurrentWeapon` _weaponslot02)
        (goto _label)))))

(event `Key|Three`
  (params (Key :type "Key Structure"))
  (bind _weaponslot03 (`self.WeaponSlot03`))
  ;[1 0 0] Key Bindings to Equip Weapons After They've Been Initially Picked Up
  (:`Pressed`
    (if (`self.is3rdSlotFilled?`)
      (if (not (== (`self.CurrentWeapon`) (`self.WeaponSlot03`)))
        (`self.EquipWeapon` _weaponslot03)
        (set `self.CurrentWeapon` _weaponslot03)
        (goto _label)))))

(event `Key|Four`
  (params (Key :type "Key Structure"))
  (bind _weaponslot04 (`self.WeaponSlot04`))
  ;[1 0 0] Key Bindings to Equip Weapons After They've Been Initially Picked Up
  (:`Pressed`
    (if (`self.is4thSlotFilled?`)
      (if (not (== (`self.CurrentWeapon`) (`self.WeaponSlot04`)))
        (`self.EquipWeapon` _weaponslot04)
        (set `self.CurrentWeapon` _weaponslot04)
        (goto _label)))))

(event `Key|Five`
  (params (Key :type "Key Structure"))
  (bind _weaponslot05 (`self.WeaponSlot05`))
  ;[1 0 0] Key Bindings to Equip Weapons After They've Been Initially Picked Up
  (:`Pressed`
    (if (`self.is5thSlotFilled?`)
      (if (not (== (`self.CurrentWeapon`) (`self.WeaponSlot05`)))
        (`self.EquipWeapon` _weaponslot05)
        (set `self.CurrentWeapon` _weaponslot05)
        (goto _label)))))

(event `Key|Six`
  (params (Key :type "Key Structure"))
  (bind _weaponslot06 (`self.WeaponSlot06`))
  ;[1 0 0] Key Bindings to Equip Weapons After They've Been Initially Picked Up
  (:`Pressed`
    (if (`self.is6thSlotFilled?`)
      (if (not (== (`self.CurrentWeapon`) (`self.WeaponSlot06`)))
        (`self.EquipWeapon` _weaponslot06)
        (set `self.CurrentWeapon` _weaponslot06)
        (goto _label)))))

(event `InputAction|Interact`
  (params (Key :type "Key Structure"))
  (bind _camera (`self.Camera`))
  (bind _returnvalue (`SceneComponent.K2_GetComponentLocation` _camera))
  ;[1 0 0] Draws Line Trace to Check if Trying to Interact with ammo or Weapon Pick Ups
  (:`Pressed`
    (bind (_outhit _returnvalue_2) (`KismetSystemLibrary.LineTraceSingle` _returnvalue (+ _returnvalue (* (`SceneComponent.GetForwardVector` _camera) 200.0)) "TraceTypeQuery1"))
    (if _returnvalue_2
      (`|ExecutionSequence`
        (:`then_0`
          (switch `/Game/FPSGame/Data/E_Loadout` (`self.Loadout`) ; Can't grab ammo without weapon
            (:`NewEnumerator1`
              (bind (_bblockinghit _binitialoverlap _time _distance _location _impactpoint _normal _impactnormal _physmat _hitactor) (`GameplayStatics.BreakHitResult` _outhit))
              (bind _asammo_pick_up_base (cast `/Game/FPSGame/Interactable/Ammo/AmmoPickUpBase` _hitactor))
              (`/Game/FPSGame/Interactable/Ammo/AmmoPickUpBase.PickUpAmmo` _asammo_pick_up_base))))
        (:`then_1`
          (bind _asweapon_pickup_base (cast `/Game/FPSGame/Interactable/Weapons/WeaponPickupBase` _hitactor))
          (`/Game/FPSGame/Interactable/Weapons/WeaponPickupBase.InteractedWithWeapon` _asweapon_pickup_base))))))

(event `InputAction|Reload`
  (params (Key :type "Key Structure"))
  (:`Pressed`
    (switch `/Game/FPSGame/Data/E_Loadout` (`self.Loadout`)
      (:`NewEnumerator1`
        (bind _returnvalue (`/Game/FPSGame/Weapons/WeaponBase.isMagFullOrEmpty?` (`self.CurrentWeapon`)))
        (if _returnvalue
          (if (`self.isSprinting?`)
            (`self.MovementStopped`))
          ;[1 0 0] Stops gun from shooting during reload
          (if (`/Game/FPSGame/Weapons/WeaponBase.isFiring?` (`self.CurrentWeapon`))
            (`/Game/FPSGame/Weapons/WeaponBase.StopShooting` (`self.CurrentWeapon`)))
          (`self.Reload`))))))

(event `InputAction|Fire`
  (params (Key :type "Key Structure"))
  ;[1 0 0] Disables shooting while sprinting
  (:`Pressed`
    (switch `/Game/FPSGame/Data/E_Loadout` (`self.Loadout`)
      (:`NewEnumerator1`
        (if (not (`self.isWeaponFireLoading?`))
          (if (`self.isSprinting?`)
            (`self.MovementStopped`))
          (`self.Fire`)))))
  (:`Released`
    (switch `/Game/FPSGame/Data/E_Loadout` (`self.Loadout`)
      (:`NewEnumerator1`
        (`/Game/FPSGame/Weapons/WeaponBase.StopShooting` (`self.CurrentWeapon`))))))

(event `InputAction|Aim`
  (params (Key :type "Key Structure"))
  (bind _loadout (`self.Loadout`))
  (bind _charactermovement (`self.CharacterMovement`))
  (:`Pressed`
    (if (not (`self.isReloading?`))
      (set `self.isAiming?` true)
      (`self.AimEnter`)
      (`self.MovementStopped`)
      ;[1 0 0] Slows player down when aiming
      (switch `/Game/FPSGame/Data/E_Loadout` _loadout
        (:`NewEnumerator1`
          (set `CharacterMovementComponent.MaxWalkSpeed` (`self.AimingWalkSpeed`) _charactermovement)))))
  (:`Released`
    (set `self.isAiming?` false)
    (`self.AimExit`)
    (switch `/Game/FPSGame/Data/E_Loadout` _loadout
      (:`NewEnumerator1`
        (set `CharacterMovementComponent.MaxWalkSpeed` (`self.MaxWalkSpeed`) _charactermovement)))))

(fn `AimFieldOfView`
  (if (`self.isAiming?`)
    ;[1 0 0] Changes FOV if Aiming Weapon
    (`CameraComponent.SetFieldOfView` (`self.Camera`) (`KismetMathLibrary.FInterpTo` (`CameraComponent.FieldOfView` (`self.Camera`)) (`/Game/FPSGame/Weapons/WeaponBase.AimFieldOfView` (`self.CurrentWeapon`)) (`GameplayStatics.GetWorldDeltaSeconds`) 10.0))
    (else
      (`CameraComponent.SetFieldOfView` (`self.Camera`) (`KismetMathLibrary.FInterpTo` (`CameraComponent.FieldOfView` (`self.Camera`)) 90.0 (`GameplayStatics.GetWorldDeltaSeconds`) 10.0)))))

(fn `HideAndShowWeaponMesh`
  (params (Weapon :type "/Game/FPSGame/Weapons/WeaponBase Object Reference"))
  (locals (LocalCurrentWeapon :type "/Game/FPSGame/Weapons/WeaponBase Object Reference"))
  (bind _weaponslot05 (`self.WeaponSlot05`))
  (bind _weaponslot06 (`self.WeaponSlot06`))
  (bind _weaponslot01 (`self.WeaponSlot01`))
  (bind _weaponslot02 (`self.WeaponSlot02`))
  (bind _weaponslot03 (`self.WeaponSlot03`))
  (bind _weaponslot04 (`self.WeaponSlot04`))
  (set `local.LocalCurrentWeapon` Weapon)
  ;[1 0 0] Hides Currently Equipped Weapon Mesh
  (`/Engine/EditorBlueprintResources/StandardMacros.IsValid` _weaponslot01
    (:`Is Valid`
      (`self.SetActorHiddenInGame` _weaponslot01 true))
    (:`Is Not Valid`
      _))
  (`/Engine/EditorBlueprintResources/StandardMacros.IsValid` _weaponslot02
    (:`Is Valid`
      (`self.SetActorHiddenInGame` _weaponslot02 true))
    (:`Is Not Valid`
      _))
  (`/Engine/EditorBlueprintResources/StandardMacros.IsValid` _weaponslot03
    (:`Is Valid`
      (`self.SetActorHiddenInGame` _weaponslot03 true))
    (:`Is Not Valid`
      _))
  (`/Engine/EditorBlueprintResources/StandardMacros.IsValid` _weaponslot04
    (:`Is Valid`
      (`self.SetActorHiddenInGame` _weaponslot04 true))
    (:`Is Not Valid`
      _))
  (`/Engine/EditorBlueprintResources/StandardMacros.IsValid` _weaponslot05
    (:`Is Valid`
      (`self.SetActorHiddenInGame` _weaponslot05 true))
    (:`Is Not Valid`
      _))
  (`/Engine/EditorBlueprintResources/StandardMacros.IsValid` _weaponslot06
    (:`Is Valid`
      (`self.SetActorHiddenInGame` _weaponslot06 true))
    (:`Is Not Valid`
      _))
  ;[1 0 0] Shows Currently Equipped Weapon Mesh
  (if (== (`local.LocalCurrentWeapon`) (`self.WeaponSlot01`))
    (`self.SetActorHiddenInGame` (`self.WeaponSlot01`) false)
    (elif (== (`local.LocalCurrentWeapon`) (`self.WeaponSlot02`))
      (`self.SetActorHiddenInGame` (`self.WeaponSlot02`) false)
      (elif (== (`local.LocalCurrentWeapon`) (`self.WeaponSlot03`))
        (`self.SetActorHiddenInGame` (`self.WeaponSlot03`) false)
        (elif (== (`local.LocalCurrentWeapon`) (`self.WeaponSlot04`))
          (`self.SetActorHiddenInGame` (`self.WeaponSlot04`) false)
          (elif (== (`local.LocalCurrentWeapon`) (`self.WeaponSlot05`))
            (`self.SetActorHiddenInGame` (`self.WeaponSlot05`) false)
            (elif (== (`local.LocalCurrentWeapon`) (`self.WeaponSlot06`))
              (`self.SetActorHiddenInGame` (`self.WeaponSlot06`) false))))))))

(fn `SpawnWeapon`
  (params (Weapon :type "/Game/FPSGame/Weapons/WeaponBase Class Reference"))
  (returns (ReturnWeapon :type "/Game/FPSGame/Weapons/WeaponBase Object Reference"))
  (locals (LocalWeapon :type "/Game/FPSGame/Weapons/WeaponBase Class Reference"))
  ;[1 0 0] Spawns Weapon Actor in Player's Hands and Assigns Weapon Slot
  (set `local.LocalWeapon` Weapon)
  (if (not (`self.is1stSlotFilled?`))
    (bind _returnvalue (`|SpawnActorFromClass` (`local.LocalWeapon`) (`self.GetTransform`) "Undefined" "OverrideRootScale" null null))
    (bind _output_get (set `self.WeaponSlot01` _returnvalue))
    (set `self.is1stSlotFilled?` true)
    (`self.K2_AttachToComponent` _output_get (`self.PlayerArms`) (`/Game/FPSGame/Weapons/WeaponBase.SocketName` _returnvalue) "SnapToTarget" "SnapToTarget" "SnapToTarget" false)
    (bind _output_get_2 (set `self.CurrentWeapon` _output_get))
    (return _output_get_2)
    (elif (not (`self.is2ndSlotFilled?`))
      (bind _returnvalue_2 (`|SpawnActorFromClass` (`local.LocalWeapon`) (`self.GetTransform`) "Undefined" "OverrideRootScale" null null))
      (bind _output_get_3 (set `self.WeaponSlot02` _returnvalue_2))
      (set `self.is2ndSlotFilled?` true)
      (`self.K2_AttachToComponent` _output_get_3 (`self.PlayerArms`) (`/Game/FPSGame/Weapons/WeaponBase.SocketName` _returnvalue_2) "SnapToTarget" "SnapToTarget" "SnapToTarget" false)
      (bind _output_get_4 (set `self.CurrentWeapon` _output_get_3))
      (return _output_get_4)
      (elif (not (`self.is3rdSlotFilled?`))
        (bind _returnvalue_3 (`|SpawnActorFromClass` (`local.LocalWeapon`) (`self.GetTransform`) "Undefined" "OverrideRootScale" null null))
        (bind _output_get_5 (set `self.WeaponSlot03` _returnvalue_3))
        (set `self.is3rdSlotFilled?` true)
        (`self.K2_AttachToComponent` _output_get_5 (`self.PlayerArms`) (`/Game/FPSGame/Weapons/WeaponBase.SocketName` _returnvalue_3) "SnapToTarget" "SnapToTarget" "SnapToTarget" false)
        (bind _output_get_6 (set `self.CurrentWeapon` _output_get_5))
        (return _output_get_6)
        (elif (not (`self.is4thSlotFilled?`))
          (bind _returnvalue_4 (`|SpawnActorFromClass` (`local.LocalWeapon`) (`self.GetTransform`) "Undefined" "OverrideRootScale" null null))
          (bind _output_get_7 (set `self.WeaponSlot04` _returnvalue_4))
          (set `self.is4thSlotFilled?` true)
          (`self.K2_AttachToComponent` _output_get_7 (`self.PlayerArms`) (`/Game/FPSGame/Weapons/WeaponBase.SocketName` _returnvalue_4) "SnapToTarget" "SnapToTarget" "SnapToTarget" false)
          (bind _output_get_8 (set `self.CurrentWeapon` _output_get_7))
          (return _output_get_8)
          (elif (not (`self.is5thSlotFilled?`))
            (bind _returnvalue_5 (`|SpawnActorFromClass` (`local.LocalWeapon`) (`self.GetTransform`) "Undefined" "OverrideRootScale" null null))
            (bind _output_get_9 (set `self.WeaponSlot05` _returnvalue_5))
            (set `self.is5thSlotFilled?` true)
            (`self.K2_AttachToComponent` _output_get_9 (`self.PlayerArms`) (`/Game/FPSGame/Weapons/WeaponBase.SocketName` _returnvalue_5) "SnapToTarget" "SnapToTarget" "SnapToTarget" false)
            (bind _output_get_10 (set `self.CurrentWeapon` _output_get_9))
            (return _output_get_10)
            (elif (not (`self.is6thSlotFilled?`))
              (bind _returnvalue_6 (`|SpawnActorFromClass` (`local.LocalWeapon`) (`self.GetTransform`) "Undefined" "OverrideRootScale" null null))
              (bind _output_get_11 (set `self.WeaponSlot06` _returnvalue_6))
              (set `self.is6thSlotFilled?` true)
              (`self.K2_AttachToComponent` _output_get_11 (`self.PlayerArms`) (`/Game/FPSGame/Weapons/WeaponBase.SocketName` _returnvalue_6) "SnapToTarget" "SnapToTarget" "SnapToTarget" false)
              (bind _output_get_12 (set `self.CurrentWeapon` _output_get_11))
              (return _output_get_12))))))))

(fn `StartSprint`
  (if (not (`NavMovementComponent.IsFalling` (`self.CharacterMovement`)))
    (set `CharacterMovementComponent.MaxWalkSpeed` (`self.SprintSpeed`) (`self.CharacterMovement`))
    (set `self.isSprinting?` true)))

(fn `StopSprint`
  (set `CharacterMovementComponent.MaxWalkSpeed` (`self.MaxWalkSpeed`) (`self.CharacterMovement`))
  (set `self.isSprinting?` false))

(fn `UserConstructionScript`)